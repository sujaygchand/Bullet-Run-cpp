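; BP_BaseTile is a course tile actor, apparently a base for the tiles in a runner game.
; On BeginPlay it caches the first BP_CourseManager in the world, though nothing in this graph uses it.
; DestroyTile waits briefly, then nudges the BP_Runner player's max walk speed up within a clamped range.
; Despite the event's name, its DestroyActor call is disconnected, so this graph never removes the tile.
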(event Custom|DestroyTile
  ;[1 1 1] Destroys tile
  (Utilities|FlowControl|Delay 0.5)
  (bind _asbp_runner (Utilities|Casting|CastToBP_Runner (Game|GetPlayerCharacter 0)))
  (Variables|/Script/Engine.CharacterMovementComponent|SetMaxWalkSpeed (Variables|/Script/Engine.Character|GetCharacterMovement _asbp_runner) (Math|Float|Clamp(Float) (+ (Variables|/Script/Engine.CharacterMovementComponent|GetMaxWalkSpeed (Variables|/Script/Engine.Character|GetCharacterMovement _asbp_runner)) 1.0) 6e+02 1.4e+03)))

(event EventBeginPlay
  (bind _outactors (Actor|GetAllActorsOfClass "/Game/WorldBP/BP_CourseManager.BP_CourseManager_C"))
  (Variables|Default|SetCourseManager (Utilities|Array|Get(acopy) _outactors)))

(fn ConstructionScript)